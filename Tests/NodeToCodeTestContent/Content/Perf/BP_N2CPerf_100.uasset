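; BP_N2CPerf_100 is an actor Blueprint of synthetic logic named as a performance test, with no gameplay beyond printing values and changing its own variables.
; BeginPlay scales Score, rebuilds a Data struct from Score and Mode, and prints them along with the Values array.
; Two custom events, not called within this graph, exercise an enum switch, nested branches, loops, Pawn casts on the owner and a Sequence node.
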(event `self.ReceiveBeginPlay`
  (set `self.Score` (+ (* (`self.Score`) 2) (`self.Score`)))
  (set `self.Data` (make `/NodeToCodeTestContent/Perf/S_N2CPerf` (`self.Score`) (`self.Mode`)))
  (for _array_element (`self.Values`)
    (`KismetSystemLibrary.PrintString` (`KismetStringLibrary.Conv_IntToString` _array_element)))
  (set `self.Data` (make `/NodeToCodeTestContent/Perf/S_N2CPerf` (`self.Score`) (`self.Mode`)))
  (`KismetSystemLibrary.PrintString` (`KismetStringLibrary.Conv_IntToString` (`self.Score`)))
  (`KismetSystemLibrary.PrintString` (`KismetStringLibrary.Conv_IntToString` (`.Count_2_CA67CA7646E784CEABA134ACA75F67B1` (break `/NodeToCodeTestContent/Perf/S_N2CPerf` (`self.Data`)))))
  (`KismetSystemLibrary.PrintString` (`KismetStringLibrary.Conv_IntToString` (`self.Score`)))
  (`KismetSystemLibrary.PrintString` (`KismetStringLibrary.Conv_IntToString` (`self.Score`)))
  (`KismetSystemLibrary.PrintString` (`KismetStringLibrary.Conv_IntToString` (`.Count_2_CA67CA7646E784CEABA134ACA75F67B1` (break `/NodeToCodeTestContent/Perf/S_N2CPerf` (`self.Data`)))))
  (set `self.Data` (make `/NodeToCodeTestContent/Perf/S_N2CPerf` (`self.Score`) (`self.Mode`)))
  (set `self.Score` (+ (* (`self.Score`) 4) (`self.Score`)))
  (for _array_element_2 (`self.Values`)
    (`KismetSystemLibrary.PrintString` (`KismetStringLibrary.Conv_IntToString` _array_element_2))))

(event `Perf_Event_001`
  (switch `/NodeToCodeTestContent/Perf/E_N2CPerf` (`self.Mode`)
    (:`NewEnumerator0`
      (`KismetSystemLibrary.PrintString` "Perf 1"))
    (:`NewEnumerator2`
      (`KismetSystemLibrary.PrintString` (`KismetStringLibrary.Conv_IntToString` (`self.Score`)))
      (if (> (`self.Score`) 53)
        (`KismetSystemLibrary.PrintString` "Perf 2")
        (else
          (for _array_element (`self.Values`)
            (`KismetSystemLibrary.PrintString` (`KismetStringLibrary.Conv_IntToString` _array_element)))
          (`KismetSystemLibrary.PrintString` (`KismetStringLibrary.Conv_IntToString` (`.Count_2_CA67CA7646E784CEABA134ACA75F67B1` (break `/NodeToCodeTestContent/Perf/S_N2CPerf` (`self.Data`)))))
          (set `self.bReady` (not (`self.bReady`)))
          (`KismetSystemLibrary.PrintString` (`KismetStringLibrary.Conv_IntToString` (`self.Score`)))
          (cast `Pawn` (`self.GetOwner`)
            (:`then`
              (`KismetSystemLibrary.PrintString` (`KismetStringLibrary.Conv_IntToString` (`self.Score`)))
              (cast `Pawn` (`self.GetOwner`)
                (:`then`
                  (for _array_element_2 (`self.Values`)
                    (`KismetSystemLibrary.PrintString` (`KismetStringLibrary.Conv_IntToString` _array_element_2)))
                  (`KismetSystemLibrary.PrintString` (`KismetStringLibrary.Conv_IntToString` (`self.Score`))))
                (:`CastFailed`
                  (`KismetSystemLibrary.PrintString` "Perf 4"))))
            (:`CastFailed`
              (`KismetSystemLibrary.PrintString` "Perf 3"))))))))

(event `Perf_Event_002`
  (`|ExecutionSequence`
    (:`then_0`
      (`KismetSystemLibrary.PrintString` (`KismetStringLibrary.Conv_IntToString` (`self.Score`))))
    (:`then_1`
      (`KismetSystemLibrary.PrintString` "Perf 5")
      (`KismetSystemLibrary.PrintString` "Perf 6")
      (`KismetSystemLibrary.PrintString` "Perf 7"))))

(fn `UserConstructionScript`)